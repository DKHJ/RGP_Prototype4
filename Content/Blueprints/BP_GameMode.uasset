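; Game mode Blueprint that sets up local multiplayer by spawning and possessing one character per player slot when play begins.
; It gathers all PlayerStart actors and, for each index up to the max player count, finds starts tagged with that index number.
; At each match it creates a local player, spawns and possesses a BP_Player, records it in a Players array, and swaps bear or fox meshes and animations by index.
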(event `self.ReceiveBeginPlay`
  (`self.GetPlayerStartPoints`)
  (`self.SpawnPlayers`))

(fn `GetPlayerStartPoints`
  (bind _outactors (`GameplayStatics.GetAllActorsOfClass` "/Script/Engine.PlayerStart"))
  (set `self.PlayerStartArray` _outactors))

(fn `SpawnPlayers`
  (bind _index (`self.Index`))
  ;[0.4158 1 0.9701] Array is zero based, update for normal 1-4 use.
  (for _index_2 (range (`self.MaxPlayerCount`))
    (set `self.Index` _index_2)
    ;[0.4374 1 0.9901] Assign each player from the array with the player start tag
    (for _array_element (`self.PlayerStartArray`)
      (if (== (`PlayerStart.PlayerStartTag` _array_element) (`KismetStringLibrary.Conv_StringToName` (`KismetStringLibrary.Conv_IntToString` (`self.Index`))))
        ;[0.4256 1 0.9602] Spawn the BP_Player and assign the player to posses it
        (`GameplayStatics.CreatePlayer` (`self.Index`))
        (bind _returnvalue (`|SpawnActorFromClass` "/Game/Blueprints/BP_Player.BP_Player_C" (`self.GetTransform` _array_element) "Undefined" "OverrideRootScale" null null))
        (`Controller.Possess` (`GameplayStatics.GetPlayerController` _index) _returnvalue)
        ;[1 1 1] Add each unique element to the players array
        (`KismetArrayLibrary.Array_AddUnique` (`self.Players`) _returnvalue)
        ;[0.2696 0.9602 1] Change the mesh and animations based on player index
        (switch `int` _index
          (:`0`
            (`SkinnedMeshComponent.SetSkinnedAssetAndUpdate` (`Character.Mesh` _returnvalue) "/Game/Assets/Animations/Bear/Bear_IdleAnim.Bear_IdleAnim" true))
          (:`1`
            (bind _mesh (`Character.Mesh` _returnvalue))
            (`SkinnedMeshComponent.SetSkinnedAssetAndUpdate` _mesh "/Game/Assets/Animations/Fox/Fox_IdleAnim.Fox_IdleAnim" true)
            (`SkeletalMeshComponent.K2_SetAnimInstanceClass` _mesh "/Game/Assets/Animations/Fox/Fox_ANIM_BP.Fox_ANIM_BP_C")))))))

(fn `UserConstructionScript`)